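; Preview actor that renders a character's equipped items to a texture for its owning BP_ThirdPersonCharacter.
; On BeginPlay a scene capture feeds a new render target, wrapped in a dynamic material handed to that character.
; Index-based functions snap nine static mesh slots to body sockets and set their meshes from data table rows or clear them.
; Slot 7 attaches BottomMesh, but setting or removing it changes ArmorMesh.
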(event EventBeginPlay
  (bind _asbp_third_person_character (Utilities|Casting|CastToBP_ThirdPersonCharacter (Components|GetOwner)))
  (bind _returnvalue (Rendering|CreateRenderTarget2D 1024 2048 "RTF_RGBA16f" "(R=0.000000,G=0.000000,B=0.000000,A=1.000000)" true))
  (bind _output_get (Variables|/Script/Engine.SceneCaptureComponent2D|SetTextureTarget (Variables|Default|GetSceneCaptureComponent2D) _returnvalue))
  (bind _returnvalue_2 (Rendering|Material|CreateDynamicMaterialInstance "/Game/BluePrints/Inventory/RenderTarget_Mat.RenderTarget_Mat" (Utilities|String|StringToName (Utilities|String|Append (Utilities|GetDisplayName _asbp_third_person_character) (Utilities|String|ToString(Integer) (Math|Random|RandomInteger 10000)))) "None" :!class /Script/Engine.KismetMaterialLibrary))
  (Variables|/Game/ThirdPerson/Blueprints/BP_ThirdPersonCharacter.BP_ThirdPersonCharacter_C|SetRenderTargetMat _asbp_third_person_character _returnvalue_2)
  (Rendering|Material|SetTextureParameterValue _returnvalue_2 "RenderTexture" _output_get))

(fn ConstructionScript)

(fn SetMeshLocations
  (params (Array :type Array%20of%20S%20Equipment%20Structures))
  (for (_ _array_index) Array
    (switch int _array_index
      (:0
        (LocalVariables|SetlocalSocketName "Cloth")
        (LocalVariables|SetLocalMesh (Variables|Default|GetClothMesh)))
      (:1
        (LocalVariables|SetlocalSocketName "Mask")
        (LocalVariables|SetLocalMesh (Variables|Default|GetMaskMesh)))
      (:2
        (LocalVariables|SetlocalSocketName "Head")
        (LocalVariables|SetLocalMesh (Variables|Default|GetHeadMesh)))
      (:3
        (LocalVariables|SetlocalSocketName "Arm")
        (LocalVariables|SetLocalMesh (Variables|Default|GetArmMesh)))
      (:4
        (LocalVariables|SetlocalSocketName "Armor")
        (LocalVariables|SetLocalMesh (Variables|Default|GetArmorMesh)))
      (:5
        (LocalVariables|SetlocalSocketName "Weapon_L")
        (LocalVariables|SetLocalMesh (Variables|Default|GetWeapon_LMesh)))
      (:6
        (LocalVariables|SetlocalSocketName "Weapon_R")
        (LocalVariables|SetLocalMesh (Variables|Default|GetWeapon_RMesh)))
      (:7
        (LocalVariables|SetlocalSocketName "Bottom")
        (LocalVariables|SetLocalMesh (Variables|Default|GetBottomMesh)))
      (:8
        (LocalVariables|SetlocalSocketName "Shoes")
        (LocalVariables|SetLocalMesh (Variables|Default|GetShoesMesh))))
    (Transformation|AttachComponentToComponent (LocalVariables|GetLocalMesh) (Variables|Default|GetMesh) (LocalVariables|GetlocalSocketName) "SnapToTarget" "SnapToTarget" "SnapToTarget" true)))

(fn SetEquipmentMesh
  (params (Item :type Data%20Table%20Row%20Handle%20Structure) (Index :type Integer))
  (bind _returnvalue (Utilities|GetDataTableRow (.datatable Item) (.rowname Item))
    (:then
      (LocalVariables|SetLocalMesh (.Mesh (Utilities|Struct|BreakS_Inventory _returnvalue)))
      (switch int Index
        (:0
          (Components|StaticMesh|SetStaticMesh (Variables|Default|GetClothMesh) (LocalVariables|GetLocalMesh)))
        (:1
          (Components|StaticMesh|SetStaticMesh (Variables|Default|GetMaskMesh) (LocalVariables|GetLocalMesh)))
        (:2
          (Components|StaticMesh|SetStaticMesh (Variables|Default|GetHeadMesh) (LocalVariables|GetLocalMesh)))
        (:3
          (Components|StaticMesh|SetStaticMesh (Variables|Default|GetArmMesh) (LocalVariables|GetLocalMesh)))
        (:4
          (Components|StaticMesh|SetStaticMesh (Variables|Default|GetArmorMesh) (LocalVariables|GetLocalMesh)))
        (:5
          (Components|StaticMesh|SetStaticMesh (Variables|Default|GetWeapon_LMesh) (LocalVariables|GetLocalMesh)))
        (:6
          (Components|StaticMesh|SetStaticMesh (Variables|Default|GetWeapon_RMesh) (LocalVariables|GetLocalMesh)))
        (:7
          (Components|StaticMesh|SetStaticMesh (Variables|Default|GetArmorMesh) (LocalVariables|GetLocalMesh)))
        (:8
          (Components|StaticMesh|SetStaticMesh (Variables|Default|GetShoesMesh) (LocalVariables|GetLocalMesh)))))))

(fn RemoveEquipmentMesh
  (params (Selection :type Integer))
  (switch int Selection
    (:0
      (Components|StaticMesh|SetStaticMesh (Variables|Default|GetClothMesh) 0))
    (:1
      (Components|StaticMesh|SetStaticMesh (Variables|Default|GetMaskMesh) 0))
    (:2
      (Components|StaticMesh|SetStaticMesh (Variables|Default|GetHeadMesh) 0))
    (:3
      (Components|StaticMesh|SetStaticMesh (Variables|Default|GetArmMesh) 0))
    (:4
      (Components|StaticMesh|SetStaticMesh (Variables|Default|GetArmorMesh) 0))
    (:5
      (Components|StaticMesh|SetStaticMesh (Variables|Default|GetWeapon_LMesh) 0))
    (:6
      (Components|StaticMesh|SetStaticMesh (Variables|Default|GetWeapon_RMesh) 0))
    (:7
      (Components|StaticMesh|SetStaticMesh (Variables|Default|GetArmorMesh) 0))
    (:8
      (Components|StaticMesh|SetStaticMesh (Variables|Default|GetShoesMesh) 0))))