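; Backpack base actor that the player picks up and wears, holding that player's inventory slots.
; On pickup, if no backpack is equipped, it registers with the player, snaps to the mesh's back socket and stops simulating physics.
; Adding merges into the first matching stack if the item's data table row allows stacking, else fills an empty slot.
; Removal writes an "Empty" sentinel row into depleted slots; index-based removal also clears player quick slots.
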(event EventPickupInteraction
  (params (Player :type BP%20Third%20Person%20Character%20Object%20Reference))
  (bind _staticmeshcomponent (Variables|Debug|GetStaticMeshComponent))
  (Utilities|IsValid (Variables|/Game/ThirdPerson/Blueprints/BP_ThirdPersonCharacter.BP_ThirdPersonCharacter_C|GetEquipeBackPack Player)
    (:Is%20Not%20Valid
      (Variables|/Game/ThirdPerson/Blueprints/BP_ThirdPersonCharacter.BP_ThirdPersonCharacter_C|SetEquipeBackPack Player self)
      (Variables|Default|SetPlayer Player)
      (Transformation|AttachComponentToComponent (Variables|/Script/Engine.Character|GetMesh (Variables|Default|GetPlayer)) "BackPackSocket" "SnapToTarget" "SnapToTarget" "SnapToTarget" true)
      (Transformation|SetWorldScale3D _staticmeshcomponent (Variables|Default|GetDefaultScale))
      (Physics|SetSimulatePhysics _staticmeshcomponent false))))

(fn ConstructionScript)

(fn FindStack
  (params (Item :type S%20Slots%20Structure%20%28by%20ref%29))
  (bind (_array_element _array_index) (Utilities|Array|ForEachLoopwithBreak (Variables|Default|GetPlayerSlots) :!label _label)
    (:LoopBody
      (if (== (.RowName (Utilities|Struct|BreakDataTableRowHandle (.Item (Utilities|Struct|BreakS_Slots _array_element)))) (.RowName (Utilities|Struct|BreakDataTableRowHandle (.Item (Utilities|Struct|BreakS_Slots Item)))))
        (LocalVariables|SetLocalFound true)
        (LocalVariables|SetLocalIndex _array_index)
        (LocalVariables|SetLocalAmount (.Amount (Utilities|Struct|BreakS_Slots _array_element)))
        (goto _label Break)))
    (:Completed
      (return (LocalVariables|GetLocalFound) (LocalVariables|GetLocalIndex) (LocalVariables|GetLocalAmount)))))

(fn FindEmptySlot
  (bind (_array_element _array_index) (Utilities|Array|ForEachLoopwithBreak (Variables|Default|GetPlayerSlots) :!label _label)
    (:LoopBody
      (if (== (.RowName (Utilities|Struct|BreakDataTableRowHandle (.Item (Utilities|Struct|BreakS_Slots _array_element)))) "Empty")
        (LocalVariables|SetLocalFound true)
        (LocalVariables|SetLocalIndex _array_index)
        (goto _label Break)))
    (:Completed
      (return (LocalVariables|GetLocalFound) (LocalVariables|GetLocalIndex)))))

(fn RemoveAmountatIndex
  (params (Index :type Integer) (Amount :type Integer))
  (bind _playerslots (Variables|Default|GetPlayerSlots))
  (bind _playerslots_2 (Variables|Default|GetPlayerSlots))
  (bind _player (Variables|Default|GetPlayer))
  (bind _output (Utilities|Array|Get(acopy) _playerslots Index))
  (bind _returnvalue (- (.amount _output) Amount))
  (if (>= _returnvalue 0)
    (if (> _returnvalue 0)
      (Utilities|Array|SetArrayElem _playerslots_2 Index (Utilities|Struct|MakeS_Slots (.item _output) _returnvalue))
      (else
        (Utilities|IsValid _player
          (:Is%20Valid
            (Default|QuickSlotRemoval _player "Inventory" Index true))
          (:Is%20Not%20Valid
            _))
        (Utilities|Array|SetArrayElem _playerslots_2 Index (Utilities|Struct|MakeS_Slots (Utilities|Struct|MakeDataTableRowHandle "/Game/BluePrints/Inventory/ItemDataTable.ItemDataTable" "Empty") 0 ""))))
    (return true)
    (else
      (return false))))

(fn RemoveItem
  (params (Item :type S%20Slots%20Structure%20%28by%20ref%29))
  (bind (_item _amount) (Utilities|Struct|BreakS_Slots Item))
  (bind _playerslots (Variables|Default|GetPlayerSlots))
  (bind (_success _index _amount_2) (CallFunction|FindStack Item))
  (if _success
    (if (>= (- _amount_2 _amount) 0)
      (if (== (- _amount_2 _amount) 0)
        (Utilities|Array|SetArrayElem _playerslots _index (Utilities|Struct|MakeS_Slots (Utilities|Struct|MakeDataTableRowHandle "/Game/BluePrints/Inventory/ItemDataTable.ItemDataTable" "Empty") 0 ""))
        (else
          (Utilities|Array|SetArrayElem _playerslots _index (Utilities|Struct|MakeS_Slots _item (- _amount_2 _amount) ""))))
      (return true)
      (else
        (return false)))
    (else
      (return false))))

(fn AddItemtoSlot
  (params (Item :type S%20Slots%20Structure) (Index :type Integer))
  (LocalVariables|SetLocalItem Item)
  (LocalVariables|SetLocalIndex Index)
  (if (== (.RowName (Utilities|Struct|BreakDataTableRowHandle (.item (Utilities|Array|Get(acopy) (Variables|Default|GetPlayerSlots) (LocalVariables|GetLocalIndex))))) "Empty")
    (Utilities|Array|SetArrayElem (Variables|Default|GetPlayerSlots) (LocalVariables|GetLocalIndex) (LocalVariables|GetLocalItem))
    (return true)
    (else
      (bind _returnvalue (Utilities|GetDataTableRow (.DataTable (Utilities|Struct|BreakDataTableRowHandle (.item (LocalVariables|GetLocalItem)))) (.RowName (Utilities|Struct|BreakDataTableRowHandle (.item (LocalVariables|GetLocalItem)))))
        (:then
          (if (and (.CanStack (Utilities|Struct|BreakS_Inventory _returnvalue)) (== (.RowName (Utilities|Struct|BreakDataTableRowHandle (.item (Utilities|Array|Get(acopy) (Variables|Default|GetPlayerSlots) (LocalVariables|GetLocalIndex))))) (.RowName (Utilities|Struct|BreakDataTableRowHandle (.item (LocalVariables|GetLocalItem))))))
            (Utilities|Array|SetArrayElem (Variables|Default|GetPlayerSlots) (LocalVariables|GetLocalIndex) (Utilities|Struct|MakeS_Slots (.item (LocalVariables|GetLocalItem)) (+ (.amount (Utilities|Array|Get(acopy) (Variables|Default|GetPlayerSlots) (LocalVariables|GetLocalIndex))) (.amount (LocalVariables|GetLocalItem)))))
            (return true)
            (else
              (return false))))
        (:RowNotFound
          (return false))))))

(fn AddItems
  (params (Item :type S%20Slots%20Structure%20%28by%20ref%29))
  (LocalVariables|SetLocalItem Item)
  (bind (_success _index) (CallFunction|FindStack (LocalVariables|GetLocalItem)))
  (if _success
    (bind _success_2 (CallFunction|AddItemtoSlot (LocalVariables|GetLocalItem) _index))
    (if _success_2
      (return _success_2)
      (else
        _)))
  (bind (_success_3 _index_2) (CallFunction|FindEmptySlot))
  (if _success_3
    (bind _success_4 (CallFunction|AddItemtoSlot (LocalVariables|GetLocalItem) _index_2))
    (return _success_4)
    (else
      (return false))))