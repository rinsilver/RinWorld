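; Shop Blueprint that keeps its own item inventory and opens the UI_Inventory widget in the Shop position when a player interacts, registering itself as their Interactable.
; Selling adds items to that inventory, merging into the first slot with the same row name when the item's data table row allows stacking.
; Buying reduces or removes the indexed slot, with no currency handling here.
; Helpers expose the inventory and check item availability; HasSpace always returns false.
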(event EventSellItem
  (params (Item :type S%20Slots%20Structure))
  (CallFunction|AddItem Item))

(event EventBuyItem
  (params (Index :type Integer) (Item :type S%20Slots%20Structure))
  (bind _inventory (Variables|Default|GetInventory))
  (bind _output (Utilities|Array|Get(acopy) _inventory Index))
  (if (> (.amount _output) (.amount Item))
    (Utilities|Array|SetArrayElem (Variables|Default|GetInventory) Index (Utilities|Struct|MakeS_Slots (.item _output) (- (.amount _output) (.amount Item)) (.type _output)))
    (else
      (Utilities|Array|RemoveIndex (Variables|Default|GetInventory) Index))))

(event EventStartInteraction
  (params (Player :type BP%20Third%20Person%20Character%20Object%20Reference))
  (Variables|/Game/ThirdPerson/Blueprints/BP_ThirdPersonCharacter.BP_ThirdPersonCharacter_C|SetInteractable Player self)
  (Default|CreateWidget Player "/Game/BluePrints/Inventory/UI_Inventory.UI_Inventory_C" "Shop"))

(fn ConstructionScript)

(fn AddItem
  (params (S_Slots :type S%20Slots%20Structure%20%28by%20ref%29))
  (LocalVariables|SetLocalItem S_Slots)
  (bind _returnvalue (Utilities|GetDataTableRow (.DataTable (Utilities|Struct|BreakDataTableRowHandle (.Item (Utilities|Struct|BreakS_Slots (LocalVariables|GetLocalItem))))) (.RowName (Utilities|Struct|BreakDataTableRowHandle (.Item (Utilities|Struct|BreakS_Slots (LocalVariables|GetLocalItem))))))
    (:then
      (if (.CanStack (Utilities|Struct|BreakS_Inventory _returnvalue))
        (bind (_success _index) (CallFunction|FindStack (LocalVariables|GetLocalItem)))
        (if _success
          (Utilities|Array|SetArrayElem (Variables|Default|GetInventory) _index (Utilities|Struct|MakeS_Slots (.item (Utilities|Array|Get(acopy) (Variables|Default|GetInventory) _index)) (+ (.amount (Utilities|Array|Get(acopy) (Variables|Default|GetInventory) _index)) (.Amount (Utilities|Struct|BreakS_Slots (LocalVariables|GetLocalItem)))) (.type (Utilities|Array|Get(acopy) (Variables|Default|GetInventory) _index))))
          (else
            (Utilities|Array|Add (Variables|Default|GetInventory) (LocalVariables|GetLocalItem) :!label _label)))
        (else
          (goto _label))))))

(fn FindStack
  (params (Item :type S%20Slots%20Structure))
  (bind (_array_element _array_index) (Utilities|Array|ForEachLoopwithBreak (Variables|Default|GetInventory) :!label _label)
    (:LoopBody
      (if (== (.RowName (Utilities|Struct|BreakDataTableRowHandle (.Item (Utilities|Struct|BreakS_Slots _array_element)))) (.RowName (Utilities|Struct|BreakDataTableRowHandle (.Item (Utilities|Struct|BreakS_Slots Item)))))
        (LocalVariables|SetLocalFound true)
        (LocalVariables|SetLocalIndex _array_index)
        (goto _label Break)))
    (:Completed
      (if (LocalVariables|GetLocalFound)
        (return (LocalVariables|GetLocalFound) (LocalVariables|GetLocalIndex))
        (else
          (return false 0))))))

(fn HasSpace
  (params (Item :type S%20Slots%20Structure))
  (return false))

(fn IsItemAvailable
  (params (Item :type S%20Slots%20Structure) (Index :type Integer))
  (return (== (.rowname (.Item (Utilities|Struct|BreakS_Slots Item))) (.rowname (.item (Utilities|Array|Get(acopy) (Variables|Default|GetInventory) Index))))))

(fn RetrieveInventory
  (return (Variables|Default|GetInventory)))