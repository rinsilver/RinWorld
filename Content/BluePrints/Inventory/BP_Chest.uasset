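; BP_Chest is an interactable storage chest that opens the inventory widget in its "Chest" position for the interacting player.
; On BeginPlay it spawns a hidden, physics-disabled backpack actor far above the origin, resized to 30 slots, as its item store.
; Buy and sell events remove or add items in that backpack.
; Helper functions check space via empty slots or stackable stacks, verify items by row name, and return the slots.
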(event EventBeginPlay
  (bind _returnvalue (Game|SpawnActorfromClass "/Game/BluePrints/Inventory/BP_BackPackMaster.BP_BackPackMaster_C" (Math|Transform|MakeTransform "0, 0,10000.000000" "0, 0, 0" "1.000000,1.000000,1.000000") "Undefined" 0 0 0))
  (bind _output_get (Variables|Default|SetEquipBackPack _returnvalue))
  (Utilities|Array|Resize (Variables|/Game/BluePrints/Inventory/BP_BackPackMaster.BP_BackPackMaster_C|GetPlayerSlots _output_get) 30)
  (Rendering|SetActorHiddenInGame (Variables|Default|GetEquipBackPack) true)
  (Physics|SetSimulatePhysics (Variables|/Script/Engine.StaticMeshActor|GetStaticMeshComponent (Variables|Default|GetEquipBackPack)) false))

(event EventStartInteraction
  (params (Player :type BP%20Third%20Person%20Character%20Object%20Reference))
  (Variables|/Game/ThirdPerson/Blueprints/BP_ThirdPersonCharacter.BP_ThirdPersonCharacter_C|SetInteractable Player self)
  (Default|CreateWidget Player "/Game/BluePrints/Inventory/UI_Inventory.UI_Inventory_C" "Chest"))

(event EventSellItem
  (params (Item :type S%20Slots%20Structure))
  (Default|AddItems (Variables|Default|GetEquipBackPack) Item))

(event EventBuyItem
  (params (Index :type Integer) (Item :type S%20Slots%20Structure))
  (Default|RemoveAmountatIndex (Variables|Default|GetEquipBackPack) Index (.amount Item)))

(fn ConstructionScript)

(fn HasSpace
  (params (Item :type S%20Slots%20Structure))
  (bind _item (Utilities|Struct|BreakS_Slots Item))
  (bind (_datatable _rowname) (Utilities|Struct|BreakDataTableRowHandle _item))
  (bind _success (Default|FindEmptySlot (Variables|Default|GetEquipBackPack)))
  (if _success
    (return true)
    (else
      (bind _returnvalue (Utilities|GetDataTableRow _datatable _rowname)
        (:then
          (if (.CanStack (Utilities|Struct|BreakS_Inventory _returnvalue))
            (bind _success_2 (Default|FindStack (Variables|Default|GetEquipBackPack) Item))
            (if _success_2
              (return true))
            (else
              (return false))))
        (:RowNotFound
          (return false))))))

(fn IsItemAvailable
  (params (Item :type S%20Slots%20Structure) (Index :type Integer))
  (return (== (.rowname (.Item (Utilities|Struct|BreakS_Slots Item))) (.rowname (.item (Utilities|Array|Get(acopy) (Variables|/Game/BluePrints/Inventory/BP_BackPackMaster.BP_BackPackMaster_C|GetPlayerSlots (Variables|Default|GetEquipBackPack)) Index))))))

(fn RetrieveInventory
  (return (Variables|/Game/BluePrints/Inventory/BP_BackPackMaster.BP_BackPackMaster_C|GetPlayerSlots (Variables|Default|GetEquipBackPack))))