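; BP_PickupMaster is a pickup actor that gives its Item to the player who interacts with it.
; The construction script looks up the item's data table row and applies that row's mesh to the static mesh component.
; On PickupInteraction it calls AddItems on the player with "Ground" as the source, and destroys itself only if that call returns true.
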(event EventPickupInteraction
  (params (Player :type BP%20Third%20Person%20Character%20Object%20Reference))
  (bind _success (Default|AddItems Player (Variables|Default|GetItem) "Ground"))
  (if _success
    (Actor|DestroyActor)))

(fn ConstructionScript
  (bind _item (Variables|Default|GetItem))
  (bind _item_2 (Utilities|Struct|BreakS_Slots _item))
  (bind (_datatable _rowname) (Utilities|Struct|BreakDataTableRowHandle _item_2))
  (bind _returnvalue (Utilities|GetDataTableRow _datatable _rowname)
    (:then
      (Components|StaticMesh|SetStaticMesh (Variables|Debug|GetStaticMeshComponent) (.Mesh (Utilities|Struct|BreakS_Inventory _returnvalue))))))