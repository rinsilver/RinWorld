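; BP_Gate02 is an interactable double gate that swings open when the E input fires while the player is nearby.
; Box overlap by BP_ThirdPersonCharacter shows or removes the W_Interact_prompt widget and opens or closes a Gate node that filters the input.
; Pressing E briefly flags the prompt as pressed, then plays the OpenDoor timeline, rotating SphereLeft and SphereRight in opposite yaw directions, with no reverse.
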(event OnComponentBeginOverlap(Box)
  (params (OverlappedComponent :type Primitive%20Component%20Object%20Reference) (OtherActor :type Actor%20Object%20Reference) (OtherComp :type Primitive%20Component%20Object%20Reference) (OtherBodyIndex :type Integer) (bFromSweep :type Boolean) (SweepResult :type Hit%20Result%20Structure%20%28by%20ref%29))
  (Utilities|Casting|CastToBP_ThirdPersonCharacter OtherActor)
  (bind _returnvalue (UserInterface|CreateWidget "/Game/Assests/moria-gates/source/model/Widget/W_Interact_prompt.W_Interact_prompt_C"))
  (UserInterface|Viewport|AddtoViewport _returnvalue 0)
  (Utilities|FlowControl|Gate true) ; enters at Open
)

(event OnComponentEndOverlap(Box)
  (params (OverlappedComponent :type Primitive%20Component%20Object%20Reference) (OtherActor :type Actor%20Object%20Reference) (OtherComp :type Primitive%20Component%20Object%20Reference) (OtherBodyIndex :type Integer))
  (Utilities|Casting|CastToBP_ThirdPersonCharacter OtherActor)
  (Widget|RemovefromParent (stale OnComponentBeginOverlap(Box) _returnvalue))
  (Utilities|FlowControl|Gate true) ; enters at Close
)

(event Custom|OnEPressed
  (Variables|/Game/Assests/moria-gates/source/model/Widget/W_Interact_prompt.W_Interact_prompt_C|SetIsPressed (stale OnComponentBeginOverlap(Box) _returnvalue) true)
  (Utilities|FlowControl|Delay 0.3)
  (Variables|/Game/Assests/moria-gates/source/model/Widget/W_Interact_prompt.W_Interact_prompt_C|SetIsPressed (stale OnComponentBeginOverlap(Box) _returnvalue) false)
  (Development|PrintString "enter gate")
  (Utilities|FlowControl|Gate true
    (:Exit
      (bind _opentrack (Timeline|OpenDoor Play)
        (:Update
          (Transformation|SetRelativeRotation (Variables|Default|GetSphere_Left) (Math|Rotator|Lerp(Rotator) "0, 0, 0" "0,-90.000000, 0" _opentrack) false false)
          (Transformation|SetRelativeRotation (Variables|Default|GetSphere_Right) (Math|Rotator|Lerp(Rotator) "0, 0, 0" "0,90.000000, 0" _opentrack) false false))))))

(fn ConstructionScript)