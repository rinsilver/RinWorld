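; BP_MeleeWeapon is a melee weapon Blueprint that supplies attack montages, damage level and socket transforms, and handles its own visual effects.
; Regular and combo montages cycle by attack count modulo array length, with a separate charge-attack montage.
; A dynamic material created on the mesh drives the charge effect, while a skeletal animation briefly plays the trail.
; Dropping the weapon switches its mesh to physics simulation.
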(event Custom|W_Materials
  (bind _returnvalue (Rendering|Material|CreateDynamicMaterialInstance (Variables|Default|GetWeapon_Mesh) (Variables|Default|GetElement%20Index) (Variables|Default|GetSource%20Material) "None" :!class /Script/Engine.PrimitiveComponent))
  (Variables|Default|SetWeaponMaterial _returnvalue))

(event EventToggleWeaponTrail
  (params (Enable :type Boolean))
  (bind _sk_trails (Variables|Default|GetSK_Trails))
  (if Enable
    (Components|Animation|PlayAnimation _sk_trails "/Game/Particles/SwordTrails/Cube_trail/CubeAnim.CubeAnim" true)
    (Utilities|FlowControl|Delay 0.2)
    (Audio|Components|Audio|Stop _sk_trails)))

(event EventBeginPlay
  (CallFunction|WMaterials))

(fn ConstructionScript)

(event EventDropWeapon
  (bind _weapon_mesh (Variables|Default|GetWeapon_Mesh))
  (Collision|SetCollisionEnabled _weapon_mesh "PhysicsOnly")
  (Collision|SetCollisionProfileName _weapon_mesh "BlockAll" false :!class /Script/Engine.PrimitiveComponent)
  (Physics|SetSimulatePhysics _weapon_mesh true))

(event EventToggleChargeWeapon
  (params (Enable :type Boolean))
  (Rendering|Material|SetScalarParameterValue (Variables|Default|GetWeaponMaterial) "ChargeMultipiler" (select Enable 1e+01 0.0) :!class /Script/Engine.MaterialInstanceDynamic))

(fn GetAttackMontage
  (params (AttackCount :type Integer) (IsComboAttack :type Boolean))
  (bind _regularattacks (Variables|Default|GetRegularAttacks))
  (bind _comboattacks (Variables|Default|GetComboAttacks))
  (if IsComboAttack
    (return (Utilities|Array|Get(acopy) _comboattacks (Math|Integer|%(Integer) AttackCount (Utilities|Array|Length _comboattacks))))
    (else
      (return (Utilities|Array|Get(acopy) _regularattacks (Math|Integer|%(Integer) AttackCount (Utilities|Array|Length _regularattacks)))))))

(fn GetChargeMontage
  (return "/Game/Characters/Tifa_Mixamo_Root/Animation/Sword_And_Shield_Slash_Montage_ChargeAttack.Sword_And_Shield_Slash_Montage_ChargeAttack"))

(fn GetDamageLevel
  (return (Variables|Default|GetdamageLevel)))

(fn GetWeaponSocketTransform
  (params (SocketName :type Name :default "None"))
  (return (Transformation|GetSocketTransform (Variables|Default|GetWeapon_Mesh) SocketName "RTS_World")))