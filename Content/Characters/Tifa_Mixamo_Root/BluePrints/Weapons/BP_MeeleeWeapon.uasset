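; Melee weapon actor built around a WeaponMesh, with a chargeable blade material and the ability to be dropped.
; On BeginPlay it creates a dynamic instance of the Blade material, whose charge multiplier scalar ToggleChargeWeapon switches on or off.
; DropWeapon turns the mesh into a blocking, physics-simulated object.
; A helper function returns world-space transforms of named mesh sockets for callers.
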(event EventDropWeapon
  (bind _weapon_mesh (Variables|Default|GetWeapon_Mesh))
  (Collision|SetCollisionEnabled _weapon_mesh "PhysicsOnly")
  (Collision|SetCollisionProfileName _weapon_mesh "BlockAll" false :!class /Script/Engine.PrimitiveComponent)
  (Physics|SetSimulatePhysics _weapon_mesh true))

(event EventToggleChargeWeapon
  (params (Enable :type Boolean))
  (Rendering|Material|SetScalarParameterValue (Variables|Default|GetWeaponMaterial) "ChargeMultipiler" (select Enable 1e+01 0.0) :!class /Script/Engine.MaterialInstanceDynamic))

(event EventBeginPlay
  (bind _returnvalue (Rendering|Material|CreateDynamicMaterialInstance (Variables|Default|GetWeapon_Mesh) 1 "/Game/Characters/Animation_Mixamo/Chaos_Blade/Blade.Blade" "None" :!class /Script/Engine.PrimitiveComponent))
  (Variables|Default|SetWeaponMaterial _returnvalue))

(fn ConstructionScript)

(fn GetWeaponSocketTransform
  (params (SocketName :type Name :default "None"))
  (return (Transformation|GetSocketTransform (Variables|Default|GetWeapon_Mesh) SocketName "RTS_World")))