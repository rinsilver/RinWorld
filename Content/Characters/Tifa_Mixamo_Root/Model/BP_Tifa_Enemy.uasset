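; Enemy AI character Blueprint (Tifa model) that fights a locked-on target and shows its health on a widget.
; Attack mode loops via FlipFlop between timed attack phases and strafe phases with random blocking.
; Attacking moves within hit range and repeats AIAttack at random intervals while the target lives.
; When not attacking, Tick-driven strafing adds sideways input plus forward or backward input chosen by target distance.
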(event EventBeginPlay
  (|CallParentFunction)
  (CallFunction|UpdateActorDetails))

(event EventSetAnimRateScale
  (params (RateScale :type Float%20%28double-precision%29))
  (Variables|/Script/Engine.SkeletalMeshComponent|SetGlobalAnimRateScale (Variables|Character|GetMesh) RateScale))

(event EventTick
  (params (DeltaSeconds :type Float%20%28single-precision%29))
  (|CallParentFunction DeltaSeconds)
  (CallFunction|UpdateActorDetails)
  (|FightStrafing))

(event EventUpdateActorDetails
  (Class|BPIUI|UpdateProgress(Message) (UserInterface|GetUserWidgetObject (Variables|Default|GetWidget_Health)) (/ (Variables|Default|GetHealth) (Variables|Default|GetMaxHealth))))

(event Collision|EventActorBeginOverlap
  (params (OtherActor :type Actor%20Object%20Reference)))

(event EventToggleAttacking
  (params (Enable :type Boolean) (Enemys :type Actor%20Object%20Reference))
  (bind _returnvalue (Transformation|GetActorLocation Enemys))
  (bind _output_get (Variables|Default|SetAttacking Enable))
  (if _output_get
    (Utilities|FlowControl|DoOnce false :!label _label
      (:Completed
        (Utilities|IsValid Enemys :!label _label_2
          (:Is%20Valid
            (if (< (Transformation|GetDistanceTo Enemys self) (Variables|Default|GethitRange)) :!label _label_3
              (bind _alive (Class|BPIBBGirl|IsAlive(Message) Enemys))
              (if _alive
                (CallFunction|AIAttack)
                (Utilities|FlowControl|Delay (Math|Random|RandomFloatinRange 2.0 5.0))
                (if (Variables|Default|GetAttacking)
                  (goto _label_2)
                  (else
                    (goto _label Reset)))
                (else
                  (CallFunction|ToggleAttackMode false)))
              (else
                (AI|Navigation|SimpleMovetoLocation (AI|GetAIController self) (+ (* (Math|Vector|Normalize (- (Transformation|GetActorLocation) _returnvalue)) (* (Variables|Default|GethitRange) 0.6)) _returnvalue))
                (Utilities|FlowControl|Delay 2.0)
                (goto _label_3)))))))))

(event EventToggleAttackMode
  (params (Enable :type Boolean) (Enemy :type Actor%20Object%20Reference))
  (bind _output_get (Variables|Default|SetIn%20attack%20mode Enable))
  (if _output_get
    (CallFunction|Lockon Enemy true)
    (Utilities|FlowControl|DoOnce false :!label _label
      (:Completed
        (Utilities|FlowControl|FlipFlop :!label _label_2
          (:A
            (Variables|Default|SetFightStrafe 0.0)
            (CallFunction|ToggleAttacking true (Variables|Default|GetLocked%20Enemy))
            (Utilities|FlowControl|Delay (Math|Random|RandomFloatinRange 6.0 1e+01)))
          (:B
            (CallFunction|ToggleBlock (Math|Random|RandomBool))
            (Variables|Default|SetFightStrafe (Math|Random|RandomFloatinRange -0.5 0.5))
            (CallFunction|ToggleAttacking false (Variables|Default|GetLocked%20Enemy))
            (Utilities|FlowControl|Delay (Math|Random|RandomFloatinRange 4.0 8.0))))
        (if (Variables|Default|GetIn%20attack%20mode)
          (goto _label_2)
          (else
            (goto _label Reset)))))
    (else
      (CallFunction|ToggleAttacking false)
      (CallFunction|Lockon 0 false))))

(fn ConstructionScript
  (|CallParentFunction))

(fn OnAlert?
  (bind _alert (Class|BPIAI|OnAlertAI?(Message) (Pawn|GetController)))
  (return _alert))